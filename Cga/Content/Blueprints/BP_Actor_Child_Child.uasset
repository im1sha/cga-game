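; BP_Actor_Child_Child is a child actor Blueprint that overrides its parent's click and rotate events.
; When clicked, it destroys itself without calling the parent's click logic.
; Its rotate event runs the parent rotation, then toggles IsColorChanged and writes it as the "Alpha" material parameter on the Cube, switching the color each time.
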(event MouseInput|EventActorOnClicked
  (params (ButtonPressed :type Key%20Structure :default "None"))
  (Actor|DestroyActor))

(event EventCustomRotateEvent
  (|CallParentFunction)
  (if (Variables|Default|GetIsColorChanged)
    (Variables|Default|SetIsColorChanged false)
    (else
      (Variables|Default|SetIsColorChanged true)))
  (Rendering|Material|SetScalarParameterValueonMaterials (Variables|Default|GetCube) "Alpha" (Math|Conversions|ToFloat(Boolean) (Variables|Default|GetIsColorChanged))))

(fn ConstructionScript
  (|CallParentFunction))