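; Child actor Blueprint that rotates its root component in steps and can toggle a continuous spin.
; CustomRotateEvent applies a fixed rotation step, calls the parent's ActorOnClicked logic, then flips IsSpinning.
; While IsSpinning is true, Tick adds local yaw scaled by SpinSpeed and delta time for frame-rate-independent motion.
; The construction script only calls the parent's version.
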(event Custom|CustomRotateEvent
  (CallFunction|RotateForward)
  (|CallParentFunction "")
  (CallFunction|SwitchSpin))

(event EventTick
  (params (DeltaSeconds :type Float%20%28single-precision%29))
  (if (Variables|Default|GetIsSpinning)
    (Transformation|AddLocalRotation (Variables|Default|GetDefaultSceneRoot) (Math|Rotator|MakeRotator 0.0 0.0 (* DeltaSeconds (Variables|Default|GetSpinSpeed))) false false)))

(fn ConstructionScript
  (|CallParentFunction))

(fn RotateForward
  (Transformation|AddLocalRotation (Variables|Default|GetDefaultSceneRoot) "10.000000, 0,0.000000" false false))

(fn SwitchSpin
  (if (Variables|Default|GetIsSpinning)
    (Variables|Default|SetIsSpinning false)
    (else
      (Variables|Default|SetIsSpinning true))))